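; Running enemy AI character that takes point and radial damage, then ragdolls and spawns a BP_Key when its health runs out.
; Death plays a sound, applies a radial impulse, disables movement, removes its capsule and BPEnemyBase component, then destroys the actor after a delay.
; Helper functions step back and forth along a PatrolRoute spline and return attack and strafe ranges, alongside an event that sets walk speed.
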(event Custom|SetWalkSpeed
  (params (Speed :type Float%20%28double-precision%29))
  ;[0.00077 0.401 0.02197] Changes enemy movement speed
  (Variables|/Script/Engine.CharacterMovementComponent|SetMaxWalkSpeed (Variables|Character|GetCharacterMovement) Speed))

(event Custom|Ragdoll
  (params (Origin :type Vector))
  ;[0.5029 0.000304 0.008023] AI turns into an immobile ragdoll object
  (Physics|SetSimulatePhysics (Variables|Character|GetMesh) true)
  (Physics|AddRadialImpulse (Variables|Character|GetMesh) (+ Origin "0.000000,0.000000,-50.000000") 3e+02 5e+04 "RIF_Constant" false)
  (Pawn|Components|CharacterMovement|DisableMovement (Variables|Character|GetCharacterMovement))
  (Game|SpawnActorfromClass "/Game/Blueprints/BP_Key.BP_Key_C" (Math|Transform|MakeTransform (Variables|/Script/Engine.SceneComponent|GetRelativeLocation (Variables|Collision|GetCapsuleComponent)) "0, 0, 0" "1.000000,1.000000,1.000000") "Undefined" "MultiplyWithRoot" 0 0)
  ;;[0.15 0.15 0.15 0.5] TODO: STOP all the AI stuff at some point after death.
  (Utilities|FlowControl|Sequence
    (:then_0
      (Components|DestroyComponent (Variables|Default|GetBP_EnemyBase)))
    (:then_1
      (Components|DestroyComponent (Variables|Collision|GetCapsuleComponent)))
    (:then_2
      (Utilities|FlowControl|Delay 6.0)
      (Actor|DestroyActor))))

(event Game|Damage|EventPointDamage
  (params (Damage :type Float%20%28single-precision%29) (DamageType :type Damage%20Type%20Object%20Reference) (HitLocation :type Vector :default "0, 0, 0") (HitNormal :type Vector :default "0, 0, 0") (HitComponent :type Primitive%20Component%20Object%20Reference) (BoneName :type Name :default "None") (ShotFromDirection :type Vector :default "0, 0, 0") (InstigatedBy :type Controller%20Object%20Reference) (DamageCauser :type Actor%20Object%20Reference) (HitInfo :type Hit%20Result%20Structure%20%28by%20ref%29))
  ;[0.5029 0.000304 0.008023] AI takes damage when attacked by the player, and ragdolls upon death
  (Development|PrintText (Utilities|Text|FormatText "{instigator} hit me for {dmg} damage!" InstigatedBy Damage))
  (bind _output_get (Variables|Default|SetHealth (- (Variables|Default|GetHealth) Damage)))
  (if (<= _output_get 0.001)
    (Development|PrintString "I am dead!")
    (CallFunction|Ragdoll ShotFromDirection)
    (Audio|PlaySoundatLocation "/Game/Audio/SC_ImDead.SC_ImDead" (Transformation|GetActorLocation) "0, 0, 0" 1.0 1.0 0.0 0 0 0 0)))

(event Game|Damage|EventRadialDamage
  (params (DamageReceived :type Float%20%28single-precision%29) (DamageType :type Damage%20Type%20Object%20Reference) (Origin :type Vector :default "0, 0, 0") (HitInfo :type Hit%20Result%20Structure%20%28by%20ref%29) (InstigatedBy :type Controller%20Object%20Reference) (DamageCauser :type Actor%20Object%20Reference))
  ;[0.5052 0.00016 0.007773] AI takes radial damage, and ragdolls upon death
  (Development|PrintText (Utilities|Text|FormatText "{instigator} hit me for {dmg} damage!" InstigatedBy DamageReceived))
  (bind _output_get (Variables|Default|SetHealth (- (Variables|Default|GetHealth) DamageReceived)))
  (if (<= _output_get 0.001)
    (Development|PrintString "I am dead!")
    (CallFunction|Ragdoll Origin)
    (Audio|PlaySoundatLocation "/Game/Audio/SC_ImDead.SC_ImDead" (Transformation|GetActorLocation) "0, 0, 0" 1.0 1.0 0.0 0 0 0 0)))

(fn ConstructionScript)

(fn GetPatrolPointLocation
  (Variables|Default|SetPatrolIndex (+ (Variables|Default|GetPatrolIndex) (Variables|Default|GetDirection))) ; Go to "next" point
  (if (>= (Variables|Default|GetPatrolIndex) (Spline|GetNumberOfSplinePoints (Variables|/Game/AI_Blueprints/BP_PatrolRoute.BP_PatrolRoute_C|GetSpline (Variables|Default|GetPatrolRoute)))) ; Are we at the end\nof the spline?
    (Variables|Default|SetDirection -1) ; Reverse the direction
    (elif (<= (Variables|Default|GetPatrolIndex) 0) ; Are we at the beginning\nof the spline?
      (Variables|Default|SetDirection 1) ; Reverse the direction
    ))
  (return (Spline|GetLocationatSplinePoint (Variables|/Game/AI_Blueprints/BP_PatrolRoute.BP_PatrolRoute_C|GetSpline (Variables|Default|GetPatrolRoute)) (Variables|Default|GetPatrolIndex) "World")))

(fn GetIdealRange
  (return (Variables|Default|GetAttack%20Range) (Variables|Default|GetStrafe%20Range)))