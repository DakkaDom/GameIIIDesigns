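; BP_Target is a target that responds when a BP_PhysicsDisc overlaps its sphere.
; The overlap sets a Hit flag and calls GetHit, which switches the cylinder to a green material.
; GetHit then finds the BP_EnemyDoor through GetActorOfClass, increments its Points and calls CheckPoints on it.
; Hit is never reset or checked before being set, so every new disc overlap adds another point.
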(event OnComponentBeginOverlap(Sphere)
  (params (OverlappedComponent :type Primitive%20Component%20Object%20Reference) (OtherActor :type Actor%20Object%20Reference) (OtherComp :type Primitive%20Component%20Object%20Reference) (OtherBodyIndex :type Integer) (bFromSweep :type Boolean) (SweepResult :type Hit%20Result%20Structure%20%28by%20ref%29))
  (Utilities|Casting|CastToBP_PhysicsDisc OtherActor)
  (Variables|Default|SetHit true)
  (CallFunction|GetHit))

(event Custom|GetHit
  (if (Variables|Default|GetHit)
    (Rendering|Material|SetMaterial (Variables|Default|GetCylinder) 0 "/AnimationSharing/AnimSharingGreen.AnimSharingGreen")
    (bind _returnvalue (Actor|GetActorOfClass "/Game/Blueprints/BP_EnemyDoor.BP_EnemyDoor_C"))
    (bind _result (Math|Integer|IncrementInt (Variables|/Game/Blueprints/BP_EnemyDoor.BP_EnemyDoor_C|GetPoints _returnvalue))
      (:%20%20
        (Variables|/Game/Blueprints/BP_EnemyDoor.BP_EnemyDoor_C|SetPoints _returnvalue _result)
        (Default|CheckPoints _returnvalue)))))

(event EventBeginPlay)

(event Collision|EventActorBeginOverlap
  (params (OtherActor :type Actor%20Object%20Reference)))

(event EventTick
  (params (DeltaSeconds :type Float%20%28single-precision%29)))

(fn ConstructionScript)