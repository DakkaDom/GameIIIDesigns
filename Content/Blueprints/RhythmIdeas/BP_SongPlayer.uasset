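; BP_SongPlayer starts the selected song in the rhythm game and sets the beat manager's tempo to match.
; On BeginPlay it caches the first-person character, BP_BeatManager and GI_RhythmGame, printing a message if any cast fails.
; It maps the game instance's SongIndex through SongNumber to a DT_SongTable row name.
; After a brief delay, that row supplies the BPM for the beat manager and the track it spawns as 2D audio.
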(event Custom|PlaySong
  (bind _beatmanager (Variables|Default|GetBeatManager))
  (bind _output_get (Variables|Default|SetRowName (.Value (Utilities|Map|GetKeyValueByIndex (Variables|Default|GetSongNumber) (Variables|/Game/Blueprints/RhythmIdeas/GI_RhythmGame.GI_RhythmGame_C|GetSongIndex (Variables|Default|GetRhythmGame))))))
  (Utilities|FlowControl|Delay 0.1)
  (bind _returnvalue (Utilities|GetDataTableRow "/Game/SoundStuff/Data/DT_SongTable.DT_SongTable" _output_get)
    (:then
      (Variables|/Game/Blueprints/RhythmIdeas/BP_BeatManager.BP_BeatManager_C|SetBPM _beatmanager (.bpm _returnvalue))
      (Default|SetBPM _beatmanager)
      (bind _returnvalue_2 (Audio|SpawnSound2D (.currentsong _returnvalue) 0.5 1.0 0.0 0))
      (Variables|Components|SetCurrentSong _returnvalue_2))
    (:RowNotFound
      (Development|PrintString "ROW NOT FOUND" true true "(R=1.000000,G=0.031888,B=0.000000,A=1.000000)"))))

(event EventBeginPlay
  (bind _asbp_first_person_character (Utilities|Casting|CastToBP_FirstPersonCharacter (Game|GetPlayerCharacter 0))
    (:then
      (Variables|Default|SetCharacterRef _asbp_first_person_character)
      (bind _returnvalue (Actor|GetActorOfClass "/Game/Blueprints/RhythmIdeas/BP_BeatManager.BP_BeatManager_C"))
      (bind _asbp_beat_manager (Utilities|Casting|CastToBP_BeatManager _returnvalue)
        (:then
          (Variables|Default|SetBeatManager _asbp_beat_manager)
          (bind _asgi_rhythm_game (Utilities|Casting|CastToGI_RhythmGame (Game|GetGameInstance))
            (:then
              (Variables|Default|SetRhythmGame _asgi_rhythm_game)
              (CallFunction|PlaySong))
            (:CastFailed
              (Development|PrintString "Instance Cast Failure" true true "(R=1.000000,G=0.031888,B=0.000000,A=1.000000)"))))
        (:CastFailed
          (Development|PrintString "Manager Cast Failure" true true "(R=1.000000,G=0.031888,B=0.000000,A=1.000000)"))))
    (:CastFailed
      (Development|PrintString "Character Cast Failure" true true "(R=1.000000,G=0.031888,B=0.000000,A=1.000000)"))))

(fn ConstructionScript)