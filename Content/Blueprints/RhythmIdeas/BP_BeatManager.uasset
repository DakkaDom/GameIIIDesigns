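; BP_BeatManager is a rhythm prototype actor that judges whether player input lands on the beat.
; BeginPlay caches the first-person character, waits briefly, derives beat and quarter-beat intervals from BPM, adds a rhythm crosshair widget and starts a timer.
; RegisterInput prints hit or miss using CheckInput, which compares game time since BeatEnd against a timing window.
; Step and AdvanceStep are empty stubs, and nothing here updates BeatEnd.
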(event Custom|SetBPM
  ;[0 0.2038 1] BPM Setup
  (bind _output_get (Variables|Default|SetInterval (/ 6e+01 (Variables|Default|GetBPM))))
  (Variables|Default|SetSubInterval (/ _output_get 4.0))
  (Variables|Default|SetBeatStart (Utilities|Time|GetGameTimeinSeconds))
  (Utilities|FlowControl|Delay 0.2)
  (bind _output_get_2 (Variables|Default|SetInterval (/ 6e+01 (Variables|Default|GetBPM))))
  (Variables|Default|SetSubInterval (/ _output_get_2 4.0))
  (Variables|Default|SetBeatStart (Utilities|Time|GetGameTimeinSeconds))
  (bind _returnvalue (UserInterface|CreateWidget "/Game/Blueprints/WBP_RhythmCrosshair.WBP_RhythmCrosshair_C" (Game|GetPlayerController 0)))
  (bind _output_get_3 (Variables|Default|SetCrosshair _returnvalue))
  (UserInterface|Viewport|AddtoViewport _output_get_3 0)
  (CallFunction|Step)
  (Utilities|Time|SetTimerbyEvent (EventDispatchers|CreateEvent :!event Custom|AdvanceStep) 0.0))

(event Custom|RegisterInput
  (bind _onbeat (CallFunction|CheckInput))
  (bind _output_get (Variables|Default|SetOnBeat _onbeat))
  (if _output_get
    (if true
      (Development|PrintString "Hit!"))
    (else
      (Development|PrintString "Miss!"))))

(event Custom|Step)

(event Custom|AdvanceStep)

(event EventBeginPlay
  (bind _asbp_first_person_character (Utilities|Casting|CastToBP_FirstPersonCharacter (Game|GetPlayerCharacter 0)))
  (Variables|Default|SetPlayerCharRef _asbp_first_person_character)
  (Utilities|FlowControl|Delay 0.2)
  (bind _output_get (Variables|Default|SetInterval (/ 6e+01 (Variables|Default|GetBPM))))
  (Variables|Default|SetSubInterval (/ _output_get 4.0))
  (Variables|Default|SetBeatStart (Utilities|Time|GetGameTimeinSeconds))
  (bind _returnvalue (UserInterface|CreateWidget "/Game/Blueprints/WBP_RhythmCrosshair.WBP_RhythmCrosshair_C" (Game|GetPlayerController 0)))
  (bind _output_get_2 (Variables|Default|SetCrosshair _returnvalue))
  (UserInterface|Viewport|AddtoViewport _output_get_2 0)
  (CallFunction|Step)
  (Utilities|Time|SetTimerbyEvent (EventDispatchers|CreateEvent :!event Custom|AdvanceStep) 0.0))

(fn ConstructionScript)

(fn CheckInput
  (bind _returnvalue (Utilities|Time|GetGameTimeinSeconds))
  (bind _beatend (Variables|Default|GetBeatEnd))
  (bind _returnvalue_2 (- _returnvalue _beatend))
  (return (<= (Math|Float|Min(Float) _returnvalue_2 (- (Variables|Default|GetInterval) (Math|Float|%(Float) _returnvalue_2 (Variables|Default|GetInterval)))) (Variables|Default|GetBeatWindow))))