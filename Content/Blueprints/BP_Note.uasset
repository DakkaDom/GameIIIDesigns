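; BP_Note is a note actor that travels along spline tracks owned by the first-person character, apparently for a rhythm mechanic.
; BeginPlay caches the character's left and right splines.
; MoveNotes plays a timeline scaled to TimeToComplete, mapping its alpha to distance along each spline.
; Each update sets the same actor's transform to left, then right with sweep, and unconnected nodes retain earlier static-spline experiments.
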(event Custom|MoveNotes
  (bind _rightsplinetrack (Variables|Default|GetRightSplineTrack))
  (bind _leftsplinetrack (Variables|Default|GetLeftSplineTrack))
  (Components|Timeline|SetPlayRate (Variables|Default|GetNoteMovement) (/ 1.0 (Variables|Default|GetTimeToComplete)))
  (bind _notetrack (Timeline|NoteMovement PlayFromStart)
    (:Update
      (Utilities|FlowControl|Sequence
        (:then_0
          (Transformation|SetActorTransform (Math|Transform|MakeTransform (Spline|GetLocationatDistanceAlongSpline _leftsplinetrack (Math|Float|Lerp 0.0 (Spline|GetSplineLength (Variables|Default|GetLeftSplineTrack)) _notetrack) "World") (Spline|GetRotationatDistanceAlongSpline _leftsplinetrack (Math|Float|Lerp 0.0 (Spline|GetSplineLength (Variables|Default|GetLeftSplineTrack)) _notetrack) "World") "0.200000,0.200000,0.200000")))
        (:then_1
          (Transformation|SetActorTransform (Math|Transform|MakeTransform (Spline|GetLocationatDistanceAlongSpline _rightsplinetrack (Math|Float|Lerp 0.0 (Spline|GetSplineLength (Variables|Default|GetRightSplineTrack)) _notetrack) "World") (Spline|GetRotationatDistanceAlongSpline _rightsplinetrack (Math|Float|Lerp 0.0 (Spline|GetSplineLength (Variables|Default|GetRightSplineTrack)) _notetrack) "World") "0.200000,0.200000,0.200000") true))))))

(event EventBeginPlay
  (bind _returnvalue (Actor|GetActorOfClass "/Game/FirstPerson/Blueprints/BP_FirstPersonCharacter.BP_FirstPersonCharacter_C"))
  (Variables|Default|SetLeftSplineTrack (Variables|/Game/FirstPerson/Blueprints/BP_FirstPersonCharacter.BP_FirstPersonCharacter_C|GetSplineLeft _returnvalue))
  (Variables|Default|SetRightSplineTrack (Variables|/Game/FirstPerson/Blueprints/BP_FirstPersonCharacter.BP_FirstPersonCharacter_C|GetSplineRight _returnvalue))
  (Development|PrintString "Set Splines"))

(fn ConstructionScript)